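; BP_CSword is a sword weapon Blueprint that shows a timed Niagara effect on its owning player.
; SpawnEffect runs the parent version, then, if the owner is BP_CPlayer, assigns NS_Basic_10 to that player's Niagara component and activates it.
; A short one-shot timer then clears the asset and deactivates the component.
; An OnSystemFinished binding is present but never runs, so cleanup relies on the timer.
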(event Custom|커스텀이벤트
  (Class|NiagaraComponent|SetAsset (Actor|GetComponentbyClass (stale EventSpawnEffect _asbp_cplayer) "/Script/Niagara.NiagaraComponent") 0 true)
  (Components|Activation|SetActive (Actor|GetComponentbyClass (stale EventSpawnEffect _asbp_cplayer) "/Script/Niagara.NiagaraComponent") false false))

(event EventBeginPlay)

(event EventSpawnEffect
  (|CallParentFunction)
  (bind _asbp_cplayer (Utilities|Casting|CastToBP_CPlayer (Components|GetOwner)))
  (Class|NiagaraComponent|SetAsset (Actor|GetComponentbyClass _asbp_cplayer "/Script/Niagara.NiagaraComponent") "/Game/Basic_VFX/Niagara/NS_Basic_10.NS_Basic_10" true)
  (Components|Activation|SetActive (Actor|GetComponentbyClass _asbp_cplayer "/Script/Niagara.NiagaraComponent") true false)
  (Utilities|Time|SetTimerbyEvent (delegate Custom|커스텀이벤트) 2.0))

(event EventTick
  (params (DeltaSeconds :type Float%20%28single-precision%29)))

(event Collision|EventActorBeginOverlap
  (params (OtherActor :type Actor%20Object%20Reference)))

(fn ConstructionScript)